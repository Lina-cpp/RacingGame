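; BP_GameMode is a game mode that tracks the car's HP and the score and shows both on the HUD.
; On BeginPlay it creates a BP_Scores widget, keeps it as HUD and adds it to the viewport.
; UpdateHealth lowers HP by one and UpdatePoints adds one point, each writing the new value straight into the widget's Lives or Points variable.
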(event `self.ReceiveBeginPlay`
  ;[1 1 1] Add widget BP_Score aka HUD
  (bind _returnvalue (`|CreateWidget` "/Game/MyFiles/Widget/BP_Scores.BP_Scores_C"))
  (bind _output_get (set `self.HUD` _returnvalue))
  (`UserWidget.AddToViewport` _output_get 0))

(event `Update Health`
  (set `self.CurrentCarHP` (- (`self.CurrentCarHP`) 1))
  (set `/Game/MyFiles/Widget/BP_Scores.Lives` (`self.CurrentCarHP`) (`self.HUD`)))

(event `Update Points`
  ;[1 1 1] Adding points to HUD
  (set `self.CurrentPoints` (+ 1 (`self.CurrentPoints`)))
  (set `/Game/MyFiles/Widget/BP_Scores.Points` (`self.CurrentPoints`) (`self.HUD`)))

(fn `UserConstructionScript`)