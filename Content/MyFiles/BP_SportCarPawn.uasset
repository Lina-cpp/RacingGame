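; Player sports car pawn that drives through its vehicle movement component, with handbrake, upright reset, orbiting spring-arm camera and front/back camera toggle.
; Braking and handbrake switch brake-light glow through a dynamic chassis material instance.
; Speed pickups add a forward velocity impulse followed by a timed adjustment; damage and point events update the game mode.
; Game over stops the car, disables input and hides it on a loss.
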(event `InputAxis|MoveForward`
  (params (AxisValue :type "Float (single-precision)"))
  (bind _vehiclemovementcomponent (`self.VehicleMovementComponent`))
  (bind _vehiclemovementcomponent_2 (`self.VehicleMovementComponent`))
  ;[1 1 1] Movement control
  ;;[1 1 1] Forward
  (if (>= AxisValue 0.0)
    (`ChaosVehicleMovementComponent.SetThrottleInput` _vehiclemovementcomponent AxisValue)
    (`ChaosVehicleMovementComponent.SetBrakeInput` _vehiclemovementcomponent 0.0)
    (`/Engine/EditorBlueprintResources/StandardMacros.DoOnce` false :!label _label
      (:`Completed`
        (`self.BrakeLights` false)))
    (else
      (`ChaosVehicleMovementComponent.SetBrakeInput` _vehiclemovementcomponent_2 (* AxisValue -1.0))
      (`ChaosVehicleMovementComponent.SetThrottleInput` _vehiclemovementcomponent_2 0.0)
      (`self.BrakeLights` true)
      (goto _label :!via `Reset`))))

(event `InputAxis|Turn`
  (params (AxisValue :type "Float (single-precision)"))
  ;[1 1 1] Movement control
  ;;[1 1 1] Turn
  (`ChaosVehicleMovementComponent.SetSteeringInput` (`self.VehicleMovementComponent`) AxisValue))

(event `InputAction|Handbrake`
  (params (Key :type "Key Structure"))
  (bind _vehiclemovementcomponent (`self.VehicleMovementComponent`))
  ;[1 1 1] Movement control
  ;;[1 1 1] Handbrake (spacebar)
  (:`Pressed`
    (`ChaosVehicleMovementComponent.SetHandbrakeInput` _vehiclemovementcomponent true)
    (`self.BrakeLights` true))
  (:`Released`
    (`ChaosVehicleMovementComponent.SetHandbrakeInput` _vehiclemovementcomponent false)
    (`self.BrakeLights` false)))

(event `InputAction|ResetCar`
  (params (Key :type "Key Structure"))
  (bind (_returnvalue_roll _returnvalue_pitch _returnvalue_yaw) (`KismetMathLibrary.BreakRotator` (`self.K2_GetActorRotation`)))
  ;[1 1 1] Car reset (Y)
  (:`Pressed`
    (`self.K2_SetActorTransform` (`KismetMathLibrary.MakeTransform` (+ (`self.K2_GetActorLocation`) (0.0 0.0 50.0)) (`KismetMathLibrary.MakeRotator` 0.0 0.0 _returnvalue_yaw)) false true)
    (`PrimitiveComponent.SetPhysicsAngularVelocityInDegrees` (`self.Mesh`) (0.0 0.0 0.0) false "None")
    (`PrimitiveComponent.SetPhysicsLinearVelocity` (`self.Mesh`) (0.0 0.0 0.0) false "None")))

(event `InputAxis|LookRight`
  (params (AxisValue :type "Float (single-precision)"))
  (bind _springarmtpp (`self.SpringArmTPP`))
  (bind (_relativerotation_roll _relativerotation_pitch _relativerotation_yaw) (`KismetMathLibrary.BreakRotator` (`SceneComponent.RelativeRotation` (`self.SpringArmTPP`))))
  ;[1 1 1] Camera Control
  ;;[1 1 1] Camera Control turn
  (if (!= AxisValue 0.0)
    (`SceneComponent.K2_AddLocalRotation` _springarmtpp (`KismetMathLibrary.MakeRotator` 0.0 0.0 AxisValue) false false)
    (else
      (`SceneComponent.K2_SetRelativeRotation` _springarmtpp (`KismetMathLibrary.MakeRotator` 0.0 0.0 (`KismetMathLibrary.FInterpTo` _relativerotation_yaw 0.0 (`GameplayStatics.GetWorldDeltaSeconds`) 1.0)) false false))))

(event `InputAction|SwitchCamera`
  (params (Key :type "Key Structure"))
  ;[1 1 1] Camera Control
  ;;[1 1 1] Switch Camera (V)
  (:`Pressed`
    (`/Engine/EditorBlueprintResources/StandardMacros.FlipFlop`
      (:`A`
        (`ActorComponent.SetActive` (`self.FrontCamera`) true false)
        (`ActorComponent.SetActive` (`self.BackCamera`) false false)
        (set `self.bUseControllerRotationYaw` true))
      (:`B`
        (`ActorComponent.SetActive` (`self.FrontCamera`) false false)
        (`ActorComponent.SetActive` (`self.BackCamera`) true false)
        (set `self.bUseControllerRotationYaw` false)))))

(event `self.ReceiveAnyDamage`
  (params (Damage :type "Float (single-precision)") (DamageType :type "DamageType Object Reference") (InstigatedBy :type "Controller Object Reference") (DamageCauser :type "Actor Object Reference"))
  ;[1 1 1] Damage pickup - lose condition
  (set `HealthComponent.Health` (`KismetMathLibrary.FTrunc` (- (`HealthComponent.Health` (`self.Health`)) Damage)) (`self.Health`))
  ;[1 1 1] Updating Health
  (bind _asbp_game_mode (cast `/Game/MyFiles/BP_GameMode` (`GameplayStatics.GetGameMode`)))
  (`/Game/MyFiles/BP_GameMode.UpdateHealth` _asbp_game_mode))

(event `SpeedBoost_Pickup`
  ;[1 1 1] Speed pickup
  ;;[1 1 1] Increase speed
  (`PrimitiveComponent.SetPhysicsLinearVelocity` (`MovementComponent.UpdatedPrimitive` (`self.VehicleMovementComponent`)) (* (`self.GetActorForwardVector`) (`self.Speed`)) true "None")
  (`KismetSystemLibrary.K2_SetTimerDelegate` (delegate `SpeedDown`) 1.0))

(event `pickupPoints`
  ;[1 1 1] Points pickup - win condition
  (bind _asbp_game_mode (cast `/Game/MyFiles/BP_GameMode` (`GameplayStatics.GetGameMode`)))
  (`/Game/MyFiles/BP_GameMode.Update Points` _asbp_game_mode))

(event `SpeedDown`
  ;[1 1 1] Speed pickup
  ;;[1 1 1] Decrase speed
  (`PrimitiveComponent.SetPhysicsLinearVelocity` (`MovementComponent.UpdatedPrimitive` (`self.VehicleMovementComponent`)) (* (`self.GetActorForwardVector`) (`self.Speed_Down`)) true "None"))

(fn `BrakeLights`
  (params (BrakeLights :type Boolean))
  (bind _returnvalue (`KismetMaterialLibrary.CreateDynamicMaterialInstance` "/Game/Vehicles/SportsCar/Materials/MI_SportsCar_Chassis.MI_SportsCar_Chassis" "None"))
  (`PrimitiveComponent.SetMaterial` (`self.Mesh`) 1 _returnvalue)
  (if BrakeLights
    (`MaterialInstanceDynamic.SetScalarParameterValue` _returnvalue "BrakeLightPower" 200.0)
    (else
      (`MaterialInstanceDynamic.SetScalarParameterValue` _returnvalue "BrakeLightPower" 4.0))))

(fn `OnGameover`
  (params (WonGame :type Boolean))
  (`MovementComponent.StopMovementImmediately` (`self.VehicleMovementComponent`))
  (`self.DisableInput` (`GameplayStatics.GetPlayerController` 0))
  (`self.SetActorHiddenInGame` (not (`local.WonGame`))))

(fn `UserConstructionScript`)